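; Game mode for Toon Tanks that drives the start, score and end screens.
; StartGame shows the start widget, and Tick polls its GameStarted flag to create the play HUD once.
; Tick then refreshes the score text from GameScore every frame by polling, with no change event.
; EndGame adds the end widget, shows the mouse cursor and displays a win or loss message from GameWon.
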(event `self.ReceiveTick`
  (params (DeltaSeconds :type "Float (single-precision)"))
  (bind _gamescore (`self.GameScore`))
  (if (`/Game/Blueprints/Widgets/WBP_StartGameWidget.GameStarted` (stale `self.StartGame` _returnvalue))
    (if (`self.bPlayWidjet`)
      (bind _scoretext (`/Game/Blueprints/Widgets/WBP_PlayGameWidget.ScoreText` (stale _returnvalue)))
      (`TextBlock.SetText` _scoretext (`KismetTextLibrary.Conv_IntToText` _gamescore))
      (else
        (bind _returnvalue (`|CreateWidget` "/Game/Blueprints/Widgets/WBP_PlayGameWidget.WBP_PlayGameWidget_C"))
        (`UserWidget.AddToViewport` _returnvalue 0)
        (`TextBlock.SetText` _scoretext (`KismetTextLibrary.Conv_IntToText` _gamescore))
        (set `self.bPlayWidjet` true)))))

(event `self.StartGame`
  (bind _returnvalue (`|CreateWidget` "/Game/Blueprints/Widgets/WBP_StartGameWidget.WBP_StartGameWidget_C"))
  (`UserWidget.AddToViewport` _returnvalue 0))

(event `self.EndGame`
  (params (bGameWon :type Boolean))
  (bind _returnvalue (`|CreateWidget` "/Game/Blueprints/Widgets/WBP_EndGameWidget.WBP_EndGameWidget_C"))
  (set `PlayerController.bShowMouseCursor` true (`GameplayStatics.GetPlayerController` 0))
  (`UserWidget.AddToViewport` _returnvalue 0)
  (`TextBlock.SetText` (`/Game/Blueprints/Widgets/WBP_EndGameWidget.DisplayText` _returnvalue) (select `bool` bGameWon :`false` "YOU LOST" :`true` "YOU WON" :!type "Text")))

(fn `UserConstructionScript`)